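; Player-controlled rolling ball with jump, orbit camera and a coin counter, driven by Enhanced Input through IMC_PlayerBall.
; Move input applies acceleration to the Ball along world X/Y, independent of camera facing, and jump adds an upward velocity impulse without a ground check.
; Camera input rotates the SpringArm in world space by a sensitivity factor, with clamped pitch.
; CollectCoin adds a given amount to the Coins total.
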(event `self.ReceiveBeginPlay`
  (bind _asplayer_controller (cast `PlayerController` (`self.GetController`)))
  (message `EnhancedInputSubsystemInterface.AddMappingContext` (pcsubsystem `EnhancedInputLocalPlayerSubsystem` _asplayer_controller) "/Game/Input/IMC_PlayerBall.IMC_PlayerBall" 0 (struct)))

(event `self.ReceiveTick`
  (params (DeltaSeconds :type "Float (single-precision)")))

(event `EnhancedInput|/Game/Input/IA_Jump`
  (params (ActionValue :type Boolean) (ElapsedSeconds :type "Float (double-precision)") (TriggeredSeconds :type "Float (double-precision)") (InputAction :type "InputAction Object Reference" :default "/Game/Input/IA_Jump.IA_Jump"))
  (:`Started`
    (`PrimitiveComponent.AddImpulse` (`self.Ball`) (`KismetMathLibrary.MakeVector` 0.0 0.0 (`self.JumpStrength`)) "None" true)))

(event `EnhancedInput|/Game/Input/IA_Move`
  (params (ActionValue :type "Vector2D Structure") (ElapsedSeconds :type "Float (double-precision)") (TriggeredSeconds :type "Float (double-precision)") (InputAction :type "InputAction Object Reference" :default "/Game/Input/IA_Move.IA_Move"))
  (bind _movestrength (`self.MoveStrength`))
  (:`Triggered`
    (`PrimitiveComponent.AddForce` (`self.Ball`) (`KismetMathLibrary.MakeVector` (* ActionValue_X _movestrength) (* ActionValue_Y _movestrength)) "None" true)))

(event `EnhancedInput|/Game/Input/IA_Camera`
  (params (ActionValue :type "Vector2D Structure") (ElapsedSeconds :type "Float (double-precision)") (TriggeredSeconds :type "Float (double-precision)") (InputAction :type "InputAction Object Reference" :default "/Game/Input/IA_Camera.IA_Camera"))
  (bind _springarm (`self.SpringArm`))
  (bind _sensitivity (`self.Sensitivity`))
  (bind (_returnvalue_roll _returnvalue_pitch _returnvalue_yaw) (`KismetMathLibrary.BreakRotator` (`SceneComponent.K2_GetComponentRotation` _springarm)))
  (:`Triggered`
    (`SceneComponent.K2_SetWorldRotation` _springarm (`KismetMathLibrary.MakeRotator` 0.0 (`KismetMathLibrary.FClamp` (+ _returnvalue_pitch (* ActionValue_Y _sensitivity)) -70.0 10.0) (+ _returnvalue_yaw (* ActionValue_X _sensitivity))) false false)))

(fn `CollectCoin`
  (params (NumberOfCoins :type Integer))
  (set `self.Coins` (+ NumberOfCoins (`self.Coins`))))

(fn `UserConstructionScript`)